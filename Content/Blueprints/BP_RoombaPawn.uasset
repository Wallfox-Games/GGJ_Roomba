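; BP_RoombaPawn is the Roomba pawn, which blinks a spotlight and opens the pause menu.
; A looping timer with randomized initial delay calls FlashLight, which toggles the spotlight and sets a short timer to toggle it back.
; Escape or P creates the pause widget once, caches it, adds it to the viewport, switches to UI-only input with a visible cursor and pauses the game.
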(event `self.ReceiveBeginPlay`
  (`KismetSystemLibrary.K2_SetTimer` null "FlashLight" 5.0 true 0.0 3.0))

(event `Key|Escape`
  (params (Key :type "Key Structure"))
  (bind _returnvalue (`GameplayStatics.GetPlayerController` 0))
  (bind _pause_menu_reference (`self.Pause Menu Reference`))
  (:`Pressed`
    (`/Engine/EditorBlueprintResources/StandardMacros.IsValid` (`self.Pause Menu Reference`) :!label _label
      (:`Is Valid`
        _)
      (:`Is Not Valid`
        (bind _returnvalue_2 (`|CreateWidget` "/Game/UserWidgets/PauseMenu.PauseMenu_C"))
        (set `self.Pause Menu Reference` _returnvalue_2)))
    (set `PlayerController.bShowMouseCursor` true _returnvalue)
    (`WidgetBlueprintLibrary.SetInputMode_UIOnlyEx` _returnvalue _pause_menu_reference)
    (`UserWidget.AddToViewport` _pause_menu_reference 0)
    (`GameplayStatics.SetGamePaused` true)))

(event `Key|P`
  (params (Key :type "Key Structure"))
  (:`Pressed`
    (goto _label)))

(fn `FlashLight`
  (`self.ToggleSpotlight`)
  (`KismetSystemLibrary.K2_SetTimer` null "ToggleSpotlight" 0.3))

(fn `ToggleSpotlight`
  (`SceneComponent.ToggleVisibility` (`self.SpotLight`) false))

(fn `UserConstructionScript`)